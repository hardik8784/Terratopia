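; RepTestItem is a test item that changes reputation when it is interacted with.
; On BeginPlay it finds the ReputationSystem actor in the level if its RepSys reference is not already valid.
; The Interaction event calls ChangeReputationMultiplier on that system, passing the item's Name variable as the reputation type and Val as the score.
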(event `self.ReceiveBeginPlay`
  (`/Engine/EditorBlueprintResources/StandardMacros.IsValid` (`self.RepSys`)
    (:`Is Not Valid`
      (bind _returnvalue (`GameplayStatics.GetActorOfClass` "/Game/Blueprints/Reputation/ReputationSystem.ReputationSystem_C"))
      (set `self.RepSys` _returnvalue))))

(event `self.Interaction`
  (`/Engine/EditorBlueprintResources/StandardMacros.IsValid` (`self.RepSys`)
    (:`Is Valid`
      (`/Game/Blueprints/Reputation/ReputationSystem.Change Reputation Multiplier` (`self.RepSys`) (`self.Name`) (`self.Val`)))))

(fn `UserConstructionScript`)