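; Reputation system Blueprint that tracks a score per reputation type and adds them to a running Reputation total.
; The construction script sizes the ReputationType array with one slot for each reputation type enum value.
; ChangeReputationMultiplier looks up a score in the ReputationMultiplier map and, if found, overwrites that type's slot.
; ClaimReputation adds every slot to Reputation, then resets the slots to their default.
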(fn `Change Reputation Multiplier`
  (params (RepType :type "/Game/Blueprints/Reputation/ReputationType Enum" :default "NewEnumerator0") (RepScore :type "/Game/Blueprints/Reputation/ReputationMultiplier Enum" :default "NewEnumerator0"))
  (bind (_value _returnvalue) (`BlueprintMapLibrary.Map_Find` (`self.ReputationMultiplier`) RepScore))
  (if _returnvalue
    (`KismetArrayLibrary.Array_Set` (`self.ReputationType`) (`KismetMathLibrary.Conv_ByteToInt` RepType) (`KismetMathLibrary.Conv_IntToDouble` _value))))

(fn `Claim Reputation`
  (for _array_element (`self.ReputationType`)
    (set `self.Reputation` (+ _array_element (`self.Reputation`))))
  (`self.ResetReputationMultiplier`))

(fn `ResetReputationMultiplier`
  (bind _reputationtype (`self.ReputationType`))
  (for (_ _array_index) _reputationtype
    (`KismetArrayLibrary.Array_Set` _reputationtype _array_index)))

(fn `UserConstructionScript`
  (locals (Index :type Integer))
  (foreach `/Game/Blueprints/Reputation/ReputationType` false
    (:`LoopBody`
      (`KismetArrayLibrary.Array_Set` (`self.ReputationType`) (`local.Index`) 0.0 true)
      (`/Engine/EditorBlueprintResources/StandardMacros.IncrementInt` (`local.Index`)))))