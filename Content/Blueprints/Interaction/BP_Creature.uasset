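; BP_Creature is an interactable creature that gains XP and advances through stages while following the player.
; Interaction toggles a lazily created CreatureInteractionUI widget that targets this creature, switching input mode and cursor visibility.
; Tick accumulates time-scaled XP while following, then resets it at a fixed threshold and increments CurrentStage.
; Advancing out of the first stage also clears the following flag, pausing XP gain.
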(event `self.Interaction`
  (if (not (`self.UIisOpen`))
    (`self.OpenUI`)
    (else
      (`self.CloseUI`))))

(event `self.ReceiveTick`
  (params (DeltaSeconds :type "Float (single-precision)"))
  (bind _currentstage (`self.CurrentStage`))
  (if (`self.bIsFollowingPlayer`)
    (bind _output_get (set `self.Xp` (+ (* (/ DeltaSeconds (`self.SecondsToLevelUp`)) (`self.XpIncreasePerSecond`)) (`self.Xp`))))
    (if (>= _output_get 500.0)
      (set `self.Xp` 0.0)
      (if (== _currentstage 0)
        (set `self.bIsFollowingPlayer` false))
      (`/Engine/EditorBlueprintResources/StandardMacros.IncrementInt` _currentstage))))

(fn `CloseUI`
  (bind _returnvalue (`GameplayStatics.GetPlayerController` 0))
  (`Widget.RemoveFromParent` (`self.UIWidget`))
  (`WidgetBlueprintLibrary.SetInputMode_GameOnly` _returnvalue)
  (set `PlayerController.bShowMouseCursor` false _returnvalue)
  (set `self.UIisOpen` false))

(fn `OpenUI`
  (bind _returnvalue (`GameplayStatics.GetPlayerController` 0))
  (bind _uiwidget (`self.UIWidget`))
  (if (not (`KismetSystemLibrary.IsValid` (`self.UIWidget`)))
    (bind _returnvalue_2 (`|CreateWidget` "/Game/Blueprints/Interaction/CreatureInteractionUI.CreatureInteractionUI_C"))
    (set `self.UIWidget` _returnvalue_2))
  (bind _ascreature_interaction_ui (cast `/Game/Blueprints/Interaction/CreatureInteractionUI` _uiwidget))
  (set `/Game/Blueprints/Interaction/CreatureInteractionUI.TargetCreature` self _ascreature_interaction_ui)
  (`UserWidget.AddToViewport` _uiwidget 0)
  (`WidgetBlueprintLibrary.SetInputMode_GameAndUIEx` _returnvalue null)
  (set `PlayerController.bShowMouseCursor` true _returnvalue)
  (set `self.UIisOpen` true))

(fn `UserConstructionScript`)